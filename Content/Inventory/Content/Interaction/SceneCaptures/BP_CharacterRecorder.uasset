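; Character stand-in actor, filed under scene captures, that mirrors equipped armor and weapons on its own skeletal mesh.
; On BeginPlay it passes itself to the player's ThirdPersonCharacter and exposes EquipItem and UnEquipItem events.
; Equipping replaces that slot's actor with a spawned, collision-disabled copy snapped to the armor's attach socket or the weapon's unequipped socket.
; Unequipping destroys the slot's actor.
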(event `self.ReceiveBeginPlay`
  (bind _asthird_person_character (cast `/Game/ThirdPersonBP/Blueprints/ThirdPersonCharacter` (`GameplayStatics.GetPlayerCharacter` 0)))
  (message `/Game/Inventory/Content/Interaction/BPI_RecorderComm.PassReference` _asthird_person_character self))

(event `/Game/Inventory/Content/Interaction/BPI_RecorderComm.EquipItem`
  (params (ItemInfo :type "/Game/Inventory/Content/Interaction/FItemInfo Structure"))
  (`self.AttachItem` ItemInfo))

(event `/Game/Inventory/Content/Interaction/BPI_RecorderComm.UnEquipItem`
  (params (ItemInfo :type "/Game/Inventory/Content/Interaction/FItemInfo Structure"))
  (`self.UnAttachItem` ItemInfo))

(fn `AttachItem`
  (params (ItemInfo :type "/Game/Inventory/Content/Interaction/FItemInfo Structure"))
  (bind ((`ItemClass_12_4931156643E18F52BF13F6A89FB6A7B6` _itemclass) (`ItemSlot_18_5CB6A6C34730C68AF0EA2AA895A13DA3` _itemslot)) (break `/Game/Inventory/Content/Interaction/FItemInfo` ItemInfo))
  (switch `/Game/Inventory/Content/Interaction/ESlotType` _itemslot
    (:`NewEnumerator1`
      (`/Engine/EditorBlueprintResources/StandardMacros.IsValid` (`self.HeadItem`)
        (:`Is Valid`
          (`self.K2_DestroyActor` (`self.HeadItem`)))
        (:`Is Not Valid`
          _))
      (bind _returnvalue (`|SpawnActorFromClass` _itemclass (`self.GetTransform`) "AlwaysSpawn" "OverrideRootScale" null null))
      (bind _output_get (set `self.HeadItem` _returnvalue))
      (bind _asbp_base_armor (cast `/Game/Inventory/Content/Interaction/Armor/BP_BaseArmor` _output_get))
      (`self.K2_AttachToComponent` _asbp_base_armor (`self.SkeletalMesh`) (`.AttachPoint_6_FCB721174D1E2BF5BB0FB6AA19C9886A` (break `/Game/Inventory/Content/Interaction/Armor/ArmorInfo` (`/Game/Inventory/Content/Interaction/Armor/BP_BaseArmor.AmorInfo` _asbp_base_armor))) "SnapToTarget" "SnapToTarget" "SnapToTarget" true)
      (`self.SetActorEnableCollision` _asbp_base_armor false))
    (:`NewEnumerator2`
      (`/Engine/EditorBlueprintResources/StandardMacros.IsValid` (`self.TorsoItem`)
        (:`Is Valid`
          (`self.K2_DestroyActor` (`self.TorsoItem`)))
        (:`Is Not Valid`
          _))
      (bind _returnvalue_2 (`|SpawnActorFromClass` _itemclass (`self.GetTransform`) "AlwaysSpawn" "OverrideRootScale" null null))
      (bind _output_get_2 (set `self.TorsoItem` _returnvalue_2))
      (bind _asbp_base_armor_2 (cast `/Game/Inventory/Content/Interaction/Armor/BP_BaseArmor` _output_get_2))
      (`self.K2_AttachToComponent` _asbp_base_armor_2 (`self.SkeletalMesh`) (`.AttachPoint_6_FCB721174D1E2BF5BB0FB6AA19C9886A` (break `/Game/Inventory/Content/Interaction/Armor/ArmorInfo` (`/Game/Inventory/Content/Interaction/Armor/BP_BaseArmor.AmorInfo` _asbp_base_armor_2))) "SnapToTarget" "SnapToTarget" "SnapToTarget" true)
      (`self.SetActorEnableCollision` _asbp_base_armor_2 false))
    (:`NewEnumerator3`
      (`/Engine/EditorBlueprintResources/StandardMacros.IsValid` (`self.LegsItem`)
        (:`Is Valid`
          (`self.K2_DestroyActor` (`self.LegsItem`)))
        (:`Is Not Valid`
          _))
      (bind _returnvalue_3 (`|SpawnActorFromClass` _itemclass (`self.GetTransform`) "AlwaysSpawn" "OverrideRootScale" null null))
      (bind _output_get_3 (set `self.LegsItem` _returnvalue_3))
      (bind _asbp_base_armor_3 (cast `/Game/Inventory/Content/Interaction/Armor/BP_BaseArmor` _output_get_3))
      (`self.K2_AttachToComponent` _asbp_base_armor_3 (`self.SkeletalMesh`) (`.AttachPoint_6_FCB721174D1E2BF5BB0FB6AA19C9886A` (break `/Game/Inventory/Content/Interaction/Armor/ArmorInfo` (`/Game/Inventory/Content/Interaction/Armor/BP_BaseArmor.AmorInfo` _asbp_base_armor_3))) "SnapToTarget" "SnapToTarget" "SnapToTarget" true)
      (`self.SetActorEnableCollision` _asbp_base_armor_3 false))
    (:`NewEnumerator4`
      (`/Engine/EditorBlueprintResources/StandardMacros.IsValid` (`self.PrimaryWeaponItem`)
        (:`Is Valid`
          (`self.K2_DestroyActor` (`self.PrimaryWeaponItem`)))
        (:`Is Not Valid`
          _))
      (bind _returnvalue_4 (`|SpawnActorFromClass` _itemclass (`self.GetTransform`) "AlwaysSpawn" "OverrideRootScale" null null))
      (bind _output_get_4 (set `self.PrimaryWeaponItem` _returnvalue_4))
      (bind _asbp_base_weapon (cast `/Game/Inventory/Content/Interaction/Weapons/BP_BaseWeapon` _output_get_4))
      (`self.K2_AttachToComponent` _asbp_base_weapon (`self.SkeletalMesh`) (`.UnEquipSocketName_23_630F13C74673A5CA93DFDEA96C7D61DF` (break `/Game/Inventory/Content/Interaction/Weapons/WeaponInfo` (`/Game/Inventory/Content/Interaction/Weapons/BP_BaseWeapon.WeaponInfo` _asbp_base_weapon))) "SnapToTarget" "SnapToTarget" "SnapToTarget" true)
      (`self.SetActorEnableCollision` _asbp_base_weapon false))
    (:`NewEnumerator5`
      (`/Engine/EditorBlueprintResources/StandardMacros.IsValid` (`self.SecondaryWeaponItem`)
        (:`Is Valid`
          (`self.K2_DestroyActor` (`self.SecondaryWeaponItem`)))
        (:`Is Not Valid`
          _))
      (bind _returnvalue_5 (`|SpawnActorFromClass` _itemclass (`self.GetTransform`) "AlwaysSpawn" "OverrideRootScale" null null))
      (bind _output_get_5 (set `self.SecondaryWeaponItem` _returnvalue_5))
      (bind _asbp_base_weapon_2 (cast `/Game/Inventory/Content/Interaction/Weapons/BP_BaseWeapon` _output_get_5))
      (`self.K2_AttachToComponent` _asbp_base_weapon_2 (`self.SkeletalMesh`) (`.UnEquipSocketName_23_630F13C74673A5CA93DFDEA96C7D61DF` (break `/Game/Inventory/Content/Interaction/Weapons/WeaponInfo` (`/Game/Inventory/Content/Interaction/Weapons/BP_BaseWeapon.WeaponInfo` _asbp_base_weapon_2))) "SnapToTarget" "SnapToTarget" "SnapToTarget" true)
      (`self.SetActorEnableCollision` _asbp_base_weapon_2 false))
    (:`NewEnumerator6`
      (`/Engine/EditorBlueprintResources/StandardMacros.IsValid` (`self.MeleeSlotItem`)
        (:`Is Valid`
          (`self.K2_DestroyActor` (`self.MeleeSlotItem`)))
        (:`Is Not Valid`
          _))
      (bind _returnvalue_6 (`|SpawnActorFromClass` _itemclass (`self.GetTransform`) "AlwaysSpawn" "OverrideRootScale" null null))
      (bind _output_get_6 (set `self.MeleeSlotItem` _returnvalue_6))
      (bind _asbp_base_weapon_3 (cast `/Game/Inventory/Content/Interaction/Weapons/BP_BaseWeapon` _output_get_6))
      (`self.K2_AttachToComponent` _asbp_base_weapon_3 (`self.SkeletalMesh`) (`.UnEquipSocketName_23_630F13C74673A5CA93DFDEA96C7D61DF` (break `/Game/Inventory/Content/Interaction/Weapons/WeaponInfo` (`/Game/Inventory/Content/Interaction/Weapons/BP_BaseWeapon.WeaponInfo` _asbp_base_weapon_3))) "SnapToTarget" "SnapToTarget" "SnapToTarget" true)
      (`self.SetActorEnableCollision` _asbp_base_weapon_3 false))
    (:`NewEnumerator7`
      (`/Engine/EditorBlueprintResources/StandardMacros.IsValid` (`self.ThrowableSlotItem`)
        (:`Is Valid`
          (`self.K2_DestroyActor` (`self.ThrowableSlotItem`)))
        (:`Is Not Valid`
          _))
      (bind _returnvalue_7 (`|SpawnActorFromClass` _itemclass (`self.GetTransform`) "AlwaysSpawn" "OverrideRootScale" null null))
      (bind _output_get_7 (set `self.ThrowableSlotItem` _returnvalue_7))
      (bind _asbp_base_weapon_4 (cast `/Game/Inventory/Content/Interaction/Weapons/BP_BaseWeapon` _output_get_7))
      (`self.K2_AttachToComponent` _asbp_base_weapon_4 (`self.SkeletalMesh`) (`.UnEquipSocketName_23_630F13C74673A5CA93DFDEA96C7D61DF` (break `/Game/Inventory/Content/Interaction/Weapons/WeaponInfo` (`/Game/Inventory/Content/Interaction/Weapons/BP_BaseWeapon.WeaponInfo` _asbp_base_weapon_4))) "SnapToTarget" "SnapToTarget" "SnapToTarget" true)
      (`self.SetActorEnableCollision` _asbp_base_weapon_4 false))))

(fn `UnAttachItem`
  (params (ItemInfo :type "/Game/Inventory/Content/Interaction/FItemInfo Structure"))
  (switch `/Game/Inventory/Content/Interaction/ESlotType` (`.ItemSlot_18_5CB6A6C34730C68AF0EA2AA895A13DA3` (break `/Game/Inventory/Content/Interaction/FItemInfo` ItemInfo))
    (:`NewEnumerator1`
      (`self.K2_DestroyActor` (`self.HeadItem`)))
    (:`NewEnumerator2`
      (`self.K2_DestroyActor` (`self.TorsoItem`)))
    (:`NewEnumerator3`
      (`self.K2_DestroyActor` (`self.LegsItem`)))
    (:`NewEnumerator4`
      (`self.K2_DestroyActor` (`self.PrimaryWeaponItem`)))
    (:`NewEnumerator5`
      (`self.K2_DestroyActor` (`self.SecondaryWeaponItem`)))
    (:`NewEnumerator6`
      (`self.K2_DestroyActor` (`self.MeleeSlotItem`)))
    (:`NewEnumerator7`
      (`self.K2_DestroyActor` (`self.ThrowableSlotItem`)))))

(fn `UserConstructionScript`)