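; BP_BaseItem is a base interactable item that a ThirdPersonCharacter picks up into its inventory.
; On Interaction, it checks the instigating character for inventory space, passes its ItemInfo struct to the character through PickUpItemMessage, then destroys itself.
; The construction script writes the actor's own class into ItemInfo, so each subclass's item data carries its class automatically.
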(event `/Game/Inventory/Content/Interaction/BPI_Interact.Interaction`
  (params (Instigator :type "/Game/ThirdPersonBP/Blueprints/ThirdPersonCharacter Object Reference"))
  (bind _asthird_person_character (cast `/Game/ThirdPersonBP/Blueprints/ThirdPersonCharacter` Instigator))
  (if (`/Game/ThirdPersonBP/Blueprints/ThirdPersonCharacter.HasSpaceInInventory?` _asthird_person_character)
    (message `/Game/Inventory/Content/Interaction/BPI_Interact.PickUpItem` _asthird_person_character (`self.ItemInfo`))
    (`self.K2_DestroyActor`)))

(fn `UserConstructionScript`
  (bind (_iteminfo_itemtype _iteminfo_itemname _iteminfo_itemimage _iteminfo_itemclass _iteminfo_itemindex _iteminfo_itemslot _iteminfo_itemvalue) (break `/Game/Inventory/Content/Interaction/FItemInfo` (`self.ItemInfo`)))
  (`parent.UserConstructionScript`)
  (set `self.ItemInfo` (make `/Game/Inventory/Content/Interaction/FItemInfo` _iteminfo_itemtype _iteminfo_itemname _iteminfo_itemimage (`GameplayStatics.GetObjectClass` self) _iteminfo_itemindex _iteminfo_itemslot _iteminfo_itemvalue)))