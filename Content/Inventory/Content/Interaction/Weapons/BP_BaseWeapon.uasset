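; Base weapon Blueprint providing automatic fire, recoil, an aim flag and reloading, driven by a WeaponInfo struct.
; A gate and retriggerable-delay loop fires while open, tracing from the camera to aim projectiles spawned at the muzzle socket.
; Each shot spends ammo and triggers casing, bolt animation, sound and particles.
; A separate event adds camera shake and timeline-driven recoil with alternating yaw, while reloading draws on MaxAmmo with a timed lock.
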(event `Casing eject`
  (bind _skeletonmesh (`self.SkeletonMesh`))
  ;[1 1 1] CasingEject
  (`|SpawnActorFromClass` "/Game/Inventory/Content/PickUps/Blueprints/Casing.Casing_C" (`KismetMathLibrary.MakeTransform` (`SceneComponent.GetSocketLocation` _skeletonmesh "Casing") (`SceneComponent.GetSocketRotation` _skeletonmesh "Casing")) "Undefined" "OverrideRootScale" null null)
  (`SkeletalMeshComponent.PlayAnimation` (`self.SkeletonMesh`) (`.BoltAnim_53_18886ECA4EA48DAB646083823526A446` (break `/Game/Inventory/Content/Interaction/Weapons/WeaponInfo` (`self.WeaponInfo`))) false))

(event `StartFire`
  (bind _returnvalue (`GameplayStatics.GetPlayerCameraManager` 0))
  (bind _skeletonmesh (`self.SkeletonMesh`))
  (bind _returnvalue_2 (`SceneComponent.GetSocketLocation` (`self.SkeletonMesh`) "Proj"))
  (bind _returnvalue_3 (`PlayerCameraManager.GetCameraLocation` _returnvalue))
  (`|ExecutionSequence`
    (:`then_0`
      (goto _label :!via `Open`))
    (:`then_1`
      (`/Engine/EditorBlueprintResources/StandardMacros.Gate` true :!label _label
        (:`Exit`
          (`|ExecutionSequence`
            (:`then_0`
              (`KismetSystemLibrary.RetriggerableDelay` 0.1)
              (goto _label))
            (:`then_1`
              (if (<= (`.CurrentAmmo_8_D6D230694714AE84B15005BC8BA9E9B8` (break `/Game/Inventory/Content/Interaction/Weapons/WeaponInfo` (`self.WeaponInfo`))) 0)
                (`KismetSystemLibrary.PrintString` "OutOfAmmo")
                (else
                  (bind (_outhit _returnvalue_4) (`KismetSystemLibrary.LineTraceSingle` _returnvalue_3 (+ _returnvalue_3 (* (`self.GetActorForwardVector` _returnvalue) 15000.0)) "TraceTypeQuery1"))
                  (if _returnvalue_4
                    _
                    (else
                      _))
                  (bind (_bblockinghit _binitialoverlap _time _distance _location _impactpoint _normal _impactnormal _physmat _hitactor _hitcomponent _hitbonename _hititem _faceindex _tracestart _traceend) (`GameplayStatics.BreakHitResult` _outhit))
                  (`GameplayStatics.SpawnSoundAtLocation` (`.WeaponSound_44_12D3C37640FC0B06BDD0BDA11537F3A7` (break `/Game/Inventory/Content/Interaction/Weapons/WeaponInfo` (`self.WeaponInfo`))) _location (struct) 1.0 1.0 0.0 null null)
                  (`self.Casing eject`)
                  (setmembers `/Game/Inventory/Content/Interaction/Weapons/WeaponInfo` :`StructRef` (`self.WeaponInfo`) :`CurrentAmmo` (- (`.CurrentAmmo_8_D6D230694714AE84B15005BC8BA9E9B8` (break `/Game/Inventory/Content/Interaction/Weapons/WeaponInfo` (`self.WeaponInfo`))) 1))
                  (`|SpawnActorFromClass` "/Game/Inventory/Content/PickUps/ProjectileBP.ProjectileBP_C" (`KismetMathLibrary.MakeTransform` _returnvalue_2 (`KismetMathLibrary.FindLookAtRotation` _returnvalue_2 (`KismetMathLibrary.SelectVector` _impactpoint _traceend _returnvalue_4))) "Undefined" "OverrideRootScale" null null)
                  (`GameplayStatics.SpawnEmitterAtLocation` "/Game/InfinityBladeEffects/Effects/FX_Cines/cinema03/P_CIN_Dust_drag_01.P_CIN_Dust_drag_01" _location (struct) (0.5 0.5 0.5))
                  (`GameplayStatics.SpawnEmitterAttached` "/Game/InfinityBladeEffects/Effects/FX_Monsters/FX_Monster_Gruntling/Master/P_BackPack_MuzzleFlash.P_BackPack_MuzzleFlash" (`self.SkeletonMesh`) "MuzzleFlash" (`SceneComponent.GetSocketLocation` _skeletonmesh "MuzzleFlash") (`SceneComponent.GetSocketRotation` _skeletonmesh "MuzzleFlash") (0.15 0.15 0.15) "KeepWorldPosition"))))))))))

(event `StopFire`
  (goto _label :!via `Close`))

(event `RecoilAndShake`
  (params (ScaleShake :type "Float (double-precision)") (ScaleRecoil :type "Float (double-precision)"))
  (bind _returnvalue (`GameplayStatics.GetPlayerCharacter` 0))
  ;[1 1 1] Recoil
  (while (`self.CanFire`)
    (`PlayerController.ClientStartCameraShake` :`self` (`GameplayStatics.GetPlayerController` 0) :`Shake` "/Game/ThirdPersonBP/Blueprints/FireShake.FireShake_C" :`Scale` ScaleShake)
    (bind (_direction _newtrack_0) (`Timeline|Timeline_0` :!via `PlayFromStart`)
      (:`Update`
        (`Pawn.AddControllerPitchInput` _returnvalue (* _newtrack_0 ScaleRecoil))
        (`/Engine/EditorBlueprintResources/StandardMacros.FlipFlop`
          (:`A`
            (`Pawn.AddControllerYawInput` _returnvalue (* (* (`KismetMathLibrary.RandomFloatInRange` 0.0 2.0) ScaleRecoil) _newtrack_0)))
          (:`B`
            (`Pawn.AddControllerYawInput` _returnvalue (* (* ScaleRecoil (`KismetMathLibrary.RandomFloatInRange` 0.0 -2.0)) _newtrack_0))))))))

(event `StartAim`
  (set `self.isAiming` true))

(event `EndAim`
  (set `self.isAiming` false))

(event `FirePress`
  (set `self.CanFire` true)
  (if (not (`self.isReloading`))
    (`self.StartFire`)))

(event `FireRelease`
  (set `self.CanFire` false)
  (`self.StopFire`))

(event `Reloading`
  (bind ((`ClipSize_28_2788511F4C90F6E33D4B6FA98CEBEFCE` _clipsize) (`CurrentAmmo_8_D6D230694714AE84B15005BC8BA9E9B8` _currentammo)) (break `/Game/Inventory/Content/Interaction/Weapons/WeaponInfo` (`self.WeaponInfo`)))
  ;[1 1 1] Reloading
  (if (== (`.MaxAmmo_10_B808ED1E472BBF7909B4329B88360CED` (break `/Game/Inventory/Content/Interaction/Weapons/WeaponInfo` (`self.WeaponInfo`))) 0)
    (`KismetSystemLibrary.PrintString` "FindAmmo")
    (elif (== _clipsize _currentammo)
      (`KismetSystemLibrary.PrintString` "FullAmmo")
      (else
        (bind _output_get (set `self.isReloading` true))
        (if _output_get
          (`self.WeaponReload`)
          (`KismetSystemLibrary.Delay` 2.0)
          (set `self.isReloading` false))))))

(event `WeaponReload`
  (bind _needed_ammo (`self.Needed Ammo`))
  (bind _weaponinfo (`self.WeaponInfo`))
  (bind ((`ClipSize_28_2788511F4C90F6E33D4B6FA98CEBEFCE` _clipsize) (`CurrentAmmo_8_D6D230694714AE84B15005BC8BA9E9B8` _currentammo)) (break `/Game/Inventory/Content/Interaction/Weapons/WeaponInfo` (`self.WeaponInfo`)))
  (bind ((`ClipSize_28_2788511F4C90F6E33D4B6FA98CEBEFCE` _clipsize_2) (`CurrentAmmo_8_D6D230694714AE84B15005BC8BA9E9B8` _currentammo_2)) (break `/Game/Inventory/Content/Interaction/Weapons/WeaponInfo` (`self.WeaponInfo`)))
  (bind ((`MaxAmmo_10_B808ED1E472BBF7909B4329B88360CED` _maxammo)) (break `/Game/Inventory/Content/Interaction/Weapons/WeaponInfo` (`self.WeaponInfo`)))
  ;[1 1 1] WeaponReload
  (if (`self.CanFire`)
    _
    (elif (> (`.MaxAmmo_10_B808ED1E472BBF7909B4329B88360CED` (break `/Game/Inventory/Content/Interaction/Weapons/WeaponInfo` (`self.WeaponInfo`))) 0)
      (set `self.Needed Ammo` (- _clipsize _currentammo))
      (if (<= _maxammo _needed_ammo)
        (setmembers `/Game/Inventory/Content/Interaction/Weapons/WeaponInfo` :`StructRef` _weaponinfo :`CurrentAmmo` (+ _clipsize_2 _currentammo_2))
        (setmembers `/Game/Inventory/Content/Interaction/Weapons/WeaponInfo` :`StructRef` _weaponinfo :`MaxAmmo` 0)
        (else
          (setmembers `/Game/Inventory/Content/Interaction/Weapons/WeaponInfo` :`StructRef` _weaponinfo :`MaxAmmo` (- _maxammo _needed_ammo))
          (setmembers `/Game/Inventory/Content/Interaction/Weapons/WeaponInfo` :`StructRef` _weaponinfo :`CurrentAmmo` (`.ClipSize_28_2788511F4C90F6E33D4B6FA98CEBEFCE` (break `/Game/Inventory/Content/Interaction/Weapons/WeaponInfo` (`self.WeaponInfo`)))))))))

(fn `UserConstructionScript`
  (`parent.UserConstructionScript`))